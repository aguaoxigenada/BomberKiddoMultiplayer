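; Game mode for BomberKiddo that manages waves of BK_Cube bricks in the level.
; On BeginPlay it hides cubes tagged DisableAtStart and turns off their collision.
; The SpawnNewBrickWave event switches on the wave number to show and re-enable collision on the cubes tagged for that wave, so waves are revealed from pre-placed actors rather than spawned.
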(event EventBeginPlay
  ;[1 1 1] Esconde los waves que no se van a utilizar al inicio y les quita la colision
  (bind _outactors (Actor|GetAllActorsOfClasswithTag "/Script/BomberKiddo.BK_Cube" "DisableAtStart"))
  (Rendering|SetActorHiddenInGame _outactors true)
  (Collision|SetActorEnableCollision _outactors false))

(event EventSpawnNewBrickWave
  (params (waveNum :type Integer))
  ;[1 1 1] Habilita y da colision a los objetos de las Waves.
  (switch int waveNum
    (:0
      (bind _outactors (Actor|GetAllActorsOfClasswithTag "/Script/BomberKiddo.BK_Cube" "Wave2"))
      (Rendering|SetActorHiddenInGame _outactors false)
      (Collision|SetActorEnableCollision _outactors true))
    (:1
      (bind _outactors_2 (Actor|GetAllActorsOfClasswithTag "/Script/BomberKiddo.BK_Cube" "Wave3"))
      (Rendering|SetActorHiddenInGame _outactors_2 false)
      (Collision|SetActorEnableCollision _outactors_2 true))
    (:2
      (bind _outactors_3 (Actor|GetAllActorsOfClasswithTag "/Script/BomberKiddo.BK_Cube" "Wave4"))
      (Rendering|SetActorHiddenInGame _outactors_3 false)
      (Collision|SetActorEnableCollision _outactors_3 true))))

(fn ConstructionScript)