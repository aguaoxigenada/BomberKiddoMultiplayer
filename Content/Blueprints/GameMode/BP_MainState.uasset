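; BP_MainState is a game state Blueprint for BP_BomberKiddoCharacter matches, but none of its logic currently runs.
; BeginPlay, Tick, PlayerDied, the construction script and the ListOfPlayers RepNotify are all empty.
; Disconnected draft nodes copy PlayerArray into ListOfPlayers, destroy PlayerStates of players at zero life or below, and call MakeWin on player 0 based on player count.
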(event Custom|PlayerDied
  ;[1 1 1] Para otra ocacion.
)

(event EventTick
  (params (DeltaSeconds :type Float%20%28single-precision%29))
  ;[1 1 1] Otra Ocasion
)

(event EventBeginPlay)

(fn ConstructionScript)

(fn OnRepListOfPlayers)